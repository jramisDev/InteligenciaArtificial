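; BP_NPC is an NPC pawn that feeds a player reference to the blackboard of its controller.
; Three seconds after BeginPlay it writes the first player controller, rather than the player's pawn, into the "Player" key.
; After another three seconds it sets that key to an empty value, so the reference is held only briefly.
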(event EventBeginPlay
  (Utilities|FlowControl|Delay 3.0)
  (AI|Components|Blackboard|SetValueasObject (AI|GetBlackboard (Pawn|GetController)) (Utilities|Name|MakeLiteralName "Player") (Game|GetPlayerController 0))
  (Utilities|FlowControl|Delay 3.0)
  (AI|Components|Blackboard|SetValueasObject (AI|GetBlackboard (Pawn|GetController)) (Utilities|Name|MakeLiteralName "Player") 0))

(fn ConstructionScript)